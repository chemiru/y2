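; BP_yPlayerController is the Arena Battle player controller that drives the HUD and game result screens.
; On BeginPlay it creates the HUD, keeps its score widget and sets the clear score from BP_ABGameMode.
; Score and retry events update that widget.
; Game over and game clear share one path that shows the result widget, and clearing also spawns a congratulation actor at the pawn's location.
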(event EventBeginPlay
  (bind _returnvalue (UserInterface|CreateWidget "/Game/ArenaBattle/UI/Wbp_yHud.Wbp_yHud_C" (Game|GetPlayerController 0)))
  (Variables|Default|SetScoreWidget (Variables|/Game/ArenaBattle/UI/Wbp_yHud.Wbp_yHud_C|GetWbp_yPlayerScore _returnvalue))
  (UserInterface|Viewport|AddtoViewport _returnvalue 0)
  (bind _asbp_abgame_mode (Utilities|Casting|CastToBP_ABGameMode (Game|GetGameMode)))
  (Default|SetClearScore (Variables|Default|GetScoreWidget) (Variables|/Script/Y.yGameMode|GetClearScore _asbp_abgame_mode)))

(event EventOnGameRetry
  (params (NewRetryCount :type Integer))
  (Default|SetRetryCount (Variables|Default|GetScoreWidget) NewRetryCount))

(event EventOnScoreChanged
  (params (Score :type Integer))
  (Default|SetScore (Variables|Default|GetScoreWidget) Score))

(event EventOnGameOver
  (Variables|Default|SetIsSuccess false)
  (bind _returnvalue (UserInterface|CreateWidget "/Game/ArenaBattle/UI/WBP_GameResult.WBP_GameResult_C" (Game|GetPlayerController 0)))
  (UserInterface|Viewport|AddtoViewport _returnvalue 0)
  (Default|SetResult _returnvalue (Variables|Default|GetIsSuccess)))

(event EventOnGameClear
  (Variables|Default|SetIsSuccess true)
  (Utilities|FlowControl|Sequence
    (:then_0
      (bind _returnvalue (UserInterface|CreateWidget "/Game/ArenaBattle/UI/WBP_GameResult.WBP_GameResult_C" (Game|GetPlayerController 0)))
      (UserInterface|Viewport|AddtoViewport _returnvalue 0)
      (Default|SetResult _returnvalue (Variables|Default|GetIsSuccess)))
    (:then_1
      (Game|SpawnActorfromClass "/Game/ArenaBattle/Blueprint/BP_Congratulation.BP_Congratulation_C" (Math|Transform|MakeTransform (Transformation|GetActorLocation (Pawn|GetControlledPawn)) "0, 0, 0" "1.000000,1.000000,1.000000") "Undefined" "MultiplyWithRoot" 0 0))))

(fn ConstructionScript)